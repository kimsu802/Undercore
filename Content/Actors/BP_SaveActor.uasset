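; BP_SaveActor is an interactable save point that lets the player save the game.
; On Interact it refuses with a UI message if the character carries the equipped-weapon tag.
; Otherwise it shows a Yes/No confirm screen and, on confirmation, saves the current game data, pushes a notification widget and plays a sound at the actor's location.
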(event EventBeginPlay)

(event Collision|EventActorBeginOverlap
  (params (OtherActor :type Actor%20Object%20Reference)))

(event EventTick
  (params (DeltaSeconds :type Float%20%28single-precision%29)))

(event EventInteract
  (params (InCharacter :type Character%20Object%20Reference))
  (Class|UndercoreFunctionLibrary|DoesActorHaveTag InCharacter "(TagName=\"Player.Status.EquippedWeapon\")"
    (:Yes
      (Class|MainMenuUISubsystem|EnqueuePushWidget (Subsystems|GetMainMenuUISubsystem) "무기를 장착한 채로는 저장이 불가능합니다."))
    (:No
      (bind _clickedbuttontype (|PushConfirmScreen "YesNo" "" "세이브 하시겠습니까?")
        (:OnButtonClicked
          (if (Utilities|Enum|Equal(Enum) _clickedbuttontype "Confirmed")
            (Class|UndercoreFunctionLibrary|SaveCurrentGameData InCharacter)
            (Class|MainMenuUISubsystem|EnqueuePushWidget (Subsystems|GetMainMenuUISubsystem) "영엄한 기운이 느껴진다..")
            (Audio|PlaySoundatLocation "/Game/Sound/Effect/Slayer_Enchant_B1.Slayer_Enchant_B1" (Transformation|GetActorLocation) "0, 0, 0" 1.0 1.0 0.0 0 0 0 0)))))))

(fn ConstructionScript)