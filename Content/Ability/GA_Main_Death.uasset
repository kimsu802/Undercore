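; Gameplay ability for the main character's death, which ends in a return to the start menu.
; It plays a random death montage, and every montage outcome ends the ability, then after a short delay shows an OK confirm screen announcing the death.
; Ending the ability pauses animations and disables capsule collision, and the confirm button opens the start menu level.
; The UI-only input and mouse cursor nodes are unconnected.
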(event Ability|EventActivateAbility
  (|PlayMontageandWaitProxy "None" (.OutItem (Utilities|Array|Random (Variables|Default|GetMontage%20to%20Play))) 1.0 "None" true 1.0 0.0 false
    (:OnCompleted
      _)
    (:OnBlendOut
      _)
    (:OnInterrupted
      _)
    (:OnCancelled
      _))
  (Ability|EndAbility)
  (Utilities|FlowControl|Delay 2.0)
  (|PushConfirmScreen "OK" "" "사망하였습니다.. 메인 메뉴로 돌아갑니다."
    (:OnButtonClicked
      (Game|OpenLevel(byObjectReference) "/Game/MedievalDungeon/Maps/Demonstration_StartMenu.Demonstration_StartMenu"))))

(event Ability|EventOnEndAbility
  (params (bWasCancelled :type Boolean))
  (Variables|/Script/Engine.SkeletalMeshComponent|SetbPauseAnims (Class|GameplayAbility|GetOwningComponentfromActorInfo) true)
  (Collision|SetCollisionEnabled (Variables|/Script/Engine.Character|GetCapsuleComponent (Class|MainGameplayAbility|GetMainCharacterfromActorInfo)) "NoCollision"))