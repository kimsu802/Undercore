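; Main character roll gameplay ability that plays a roll montage steered by motion warping and ends when the montage finishes or is interrupted.
; After a brief delay on activation, it sets a rotation warp target from the last movement input direction.
; It offsets the character location by a level-scaled distance, traces downward to find the ground, and uses the impact point as the roll's location warp target.
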(event Ability|EventActivateAbility
  (Utilities|FlowControl|Delay 0.05)
  (CallFunction|ComputeRollDirectionandDistance)
  (|PlayMontageandWaitProxy "None" "/Game/Animations/WarriorAnimation/DKF_Hero_Roll_Montage.DKF_Hero_Roll_Montage" 1.0 "None" true 1.0 0.0 false
    (:OnCompleted
      _)
    (:OnBlendOut
      _)
    (:OnInterrupted
      _)
    (:OnCancelled
      _))
  (Ability|EndAbility))

(event Ability|EventOnEndAbility
  (params (bWasCancelled :type Boolean)))

(fn ComputeRollDirectionandDistance
  (LocalVariables|SetCachedRollingDirection (Math|Vector|Normalize (Class|Pawn|GetLastMovementInputVector (Class|MainGameplayAbility|GetMainCharacterfromActorInfo))))
  (Utilities|FlowControl|Sequence
    (:then_0
      (Class|MotionWarpingComponent|AddorUpdateWarpTargetfromLocationandRotation (Variables|/Script/UnderCore.UndercoreBaseCharacter|GetMotionWarpingComponent (Class|MainGameplayAbility|GetMainCharacterfromActorInfo)) "RollingDirection" "0, 0, 0" (Math|Rotator|MakeRotfromX (LocalVariables|GetCachedRollingDirection))))
    (:then_1
      (bind _outhit (Collision|LineTraceForObjects (+ (* (LocalVariables|GetCachedRollingDirection) (Class|UndercoreFunctionLibrary|GetScalableFloatValueatLevel (Variables|Default|GetRollingDistanceScalableFloat) (Math|Conversions|ToFloat(Integer) (Ability|GetAbilityLevel)))) (Transformation|GetActorLocation (Class|MainGameplayAbility|GetMainCharacterfromActorInfo))) (+ (+ (* (LocalVariables|GetCachedRollingDirection) (Class|UndercoreFunctionLibrary|GetScalableFloatValueatLevel (Variables|Default|GetRollingDistanceScalableFloat) (Math|Conversions|ToFloat(Integer) (Ability|GetAbilityLevel)))) (Transformation|GetActorLocation (Class|MainGameplayAbility|GetMainCharacterfromActorInfo))) (* (* (Transformation|GetActorUpVector (Class|MainGameplayAbility|GetMainCharacterfromActorInfo)) -1.0) 5e+02)) (Variables|Default|GetObject%20Types) false 0 "None"))
      (Class|MotionWarpingComponent|AddorUpdateWarpTargetfromLocationandRotation (Variables|/Script/UnderCore.UndercoreBaseCharacter|GetMotionWarpingComponent (Class|MainGameplayAbility|GetMainCharacterfromActorInfo)) "RollTargetLocation" (.ImpactPoint (Collision|BreakHitResult _outhit)) "0, 0, 0"))))