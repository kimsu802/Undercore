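; Base Gameplay Ability for enemy hit reactions, triggered by a gameplay event carrying the attacker as Instigator.
; If FaceAttacker is set, it turns the enemy toward the attacker and launches it horizontally away, scaled by LaunchPower and their separation.
; It plays a random montage, or waits briefly without one, while a material parameter enables the hit effect until the ability ends.
; It also applies the GE_Enemy_UnderAttack effect to the owner.
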(event Ability|EventActivateAbility)

(event Ability|EventOnEndAbility
  (params (bWasCancelled :type Boolean))
  (Rendering|Material|SetScalarParameterValueonMaterials (Class|GameplayAbility|GetOwningComponentfromActorInfo) "HitFxSwitch" 0.0))

(event Ability|EventActivateAbilityFromEvent
  (params (EventData :type Gameplay%20Event%20Data%20Structure%20%28by%20ref%29))
  (bind _instigator (Utilities|Struct|BreakGameplayEventData EventData))
  (bind _returnvalue (Class|UndercoreEnemyGameplayAbility|GetEnemyCharacterfromActorInfo))
  (bind _launchpower (Variables|Default|GetLaunchPower))
  (bind _returnvalue_2 (Transformation|GetActorLocation _returnvalue))
  (bind _returnvalue_3 (Transformation|GetActorLocation _instigator))
  (bind _returnvalue_4 (- _returnvalue_2 _returnvalue_3))
  (bind (_x _y) (Math|Vector|BreakVector _returnvalue_4))
  (Development|PrintString "lalala")
  (Utilities|FlowControl|Sequence
    (:then_0
      (if (Variables|Default|GetFaceAttacker)
        (Transformation|SetActorRotation (Class|UndercoreEnemyGameplayAbility|GetEnemyCharacterfromActorInfo) (Math|Rotator|FindLookatRotation _returnvalue_2 _returnvalue_3))
        (Character|LaunchCharacter _returnvalue (Math|Vector|MakeVector (* _x _launchpower) (* _y _launchpower) 0.0) false false)))
    (:then_1
      (if (Variables|Default|GetHasHitReactMontagesToPlay)
        (|PlayMontageandWaitProxy "None" (.OutItem (Utilities|Array|Random (Variables|Default|GetMontage%20to%20Play))) 1.0 "None" true 1.0 0.0 false
          (:then
            (Rendering|Material|SetScalarParameterValueonMaterials (Class|GameplayAbility|GetOwningComponentfromActorInfo) "HitFxSwitch" 1.0 :!label _label)
            (if (not (Variables|Default|GetHasHitReactMontagesToPlay))
              (Utilities|FlowControl|Delay 0.2)
              (Ability|EndAbility)))
          (:OnCompleted
            (Ability|EndAbility :!label _label_2))
          (:OnBlendOut
            (goto _label_2))
          (:OnInterrupted
            (goto _label_2))
          (:OnCancelled
            (goto _label_2)))
        (else
          (goto _label))))
    (:then_2
      (Ability|ApplyGameplayEffectSpecToOwner (Ability|MakeOutgoingGameplayEffectSpec "/Game/GameplayEffect/GE_Enemy_UnderAttack.GE_Enemy_UnderAttack_C")))))