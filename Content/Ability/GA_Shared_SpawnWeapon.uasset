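; Shared gameplay ability that spawns a configurable weapon for the avatar pawn and attaches it to the character.
; On activation it spawns the weapon class with the avatar as owner and instigator, then attaches its mesh to a configurable socket on the owning component.
; It registers the weapon by tag with the pawn combat component, optionally as the equipped weapon, and ends once that valid spawn is handled.
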(event Ability|EventActivateAbility
  (bind _returnvalue (Ability|GetAvatarActorfromActorInfo))
  (bind _as폰 (Utilities|Casting|CastToPawn _returnvalue))
  (bind _returnvalue_2 (Game|SpawnActorfromClass (Variables|Default|GetWeaponClassToSpawn) (Math|Transform|MakeTransform "0, 0, 0" "0, 0, 0" "1.000000,1.000000,1.000000") "AdjustIfPossibleButAlwaysSpawn" "MultiplyWithRoot" _returnvalue _as폰))
  (Utilities|IsValid _returnvalue_2
    (:Is%20Valid
      (Transformation|AttachComponentToComponent (Variables|/Script/UnderCore.UndercoreWeaponBase|GetWeaponMesh _returnvalue_2) (Class|GameplayAbility|GetOwningComponentfromActorInfo) (Variables|Default|GetSocketNameAttachTo) "SnapToTarget" "KeepRelative" "KeepWorld" true)
      (Class|PawnCombatComponent|RegisterSpawnedWeapon (Class|UndercoreGameplayAbility|GetPawnCombatComponentfromActorInfo) (Variables|Default|GetIn%20Weapon%20Tag%20to%20Register) _returnvalue_2 (Variables|Default|GetRegister%20as%20Equipped%20Weapon))
      (Ability|EndAbility))))

(event Ability|EventOnEndAbility
  (params (bWasCancelled :type Boolean)))