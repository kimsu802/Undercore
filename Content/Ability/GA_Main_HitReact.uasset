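; Gameplay ability that plays a directional hit reaction on the main character, activated by a gameplay event.
; It computes a front, back, left or right hit-react tag from the event's instigator and the character, then switches on that tag to pick the matching montage.
; The ability ends when the montage completes, blends out, is interrupted or is cancelled.
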(event Ability|EventActivateAbility)

(event Ability|EventOnEndAbility
  (params (bWasCancelled :type Boolean)))

(event Ability|EventActivateAbilityFromEvent
  (params (EventData :type Gameplay%20Event%20Data%20Structure%20%28by%20ref%29))
  (|SwitchGameplayTag (.ReturnValue (Class|UndercoreFunctionLibrary|ComputeHitReactDirectionTag (.Instigator (Utilities|Struct|BreakGameplayEventData EventData)) (Class|MainGameplayAbility|GetMainCharacterfromActorInfo)))
    (:Shared.Status.HitReact.Back
      (Variables|Default|SetMontage%20to%20Play "/Game/Animations/WarriorAnimation/DKF_Hero_HitReact_Back_Montage.DKF_Hero_HitReact_Back_Montage"))
    (:Shared.Status.HitReact.Front
      (Variables|Default|SetMontage%20to%20Play "/Game/Animations/WarriorAnimation/DKF_Hero_HitReact_Front_Montage.DKF_Hero_HitReact_Front_Montage"))
    (:Shared.Status.HitReact.Left
      (Variables|Default|SetMontage%20to%20Play "/Game/Animations/WarriorAnimation/DKF_Hero_HitReact_Left_Montage.DKF_Hero_HitReact_Left_Montage"))
    (:Shared.Status.HitReact.Right
      (Variables|Default|SetMontage%20to%20Play "/Game/Animations/WarriorAnimation/DKF_Hero_HitReact_Right_Montage.DKF_Hero_HitReact_Right_Montage")))
  (|PlayMontageandWaitProxy "None" (Variables|Default|GetMontage%20to%20Play) 1.0 "None" true 1.0 0.0 false
    (:OnCompleted
      _)
    (:OnBlendOut
      _)
    (:OnInterrupted
      _)
    (:OnCancelled
      _))
  (Ability|EndAbility))